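; BP_EnemyKrol is a PaperZD enemy with boosted stats that endlessly chases the player and damages the player character on sphere overlap through BPC_Stats.
; A looping timer is set at BeginPlay, and Smierc destroys the actor once dead.
; Tick uses delayed sphere traces to place short-lived, purely visual spark or fire bursts by health.
; The quarter-health branch is unreachable, nested under the at-least-half-health path.
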(event `Smierc`
  (bind _isdead (`/Game/_Cyberiada/PlayerStats/BPC_Stats.getIsDead` (`self.BPC_Stats`)))
  (if _isdead
    (`self.K2_DestroyActor`)))

(event `self.ReceiveBeginPlay`
  (bind _bpc_stats (`self.BPC_Stats`))
  (`parent.ReceiveBeginPlay`)
  (`KismetSystemLibrary.K2_SetTimerDelegate` (`|CreateDelegate` :!event `Smierc`) 0.5 true)
  (bind _output_get (set `/Game/_Cyberiada/PlayerStats/BPC_Stats.MaxHp` 190 _bpc_stats))
  (set `/Game/_Cyberiada/PlayerStats/BPC_Stats.Hp` _output_get _bpc_stats)
  (set `/Game/_Cyberiada/PlayerStats/BPC_Stats.Damage` 35 _bpc_stats)
  (`|AIMoveTo` self (0.0 0.0 0.0) (`GameplayStatics.GetPlayerCharacter` 0) 50.0 :!label _label
    (:`OnSuccess`
      (goto _label))
    (:`OnFail`
      (goto _label))))

(event `self.Sphere.OnComponentBeginOverlap`
  (params (OverlappedComponent :type "PrimitiveComponent Object Reference") (OtherActor :type "Actor Object Reference") (OtherComp :type "PrimitiveComponent Object Reference") (OtherBodyIndex :type Integer) (bFromSweep :type Boolean) (SweepResult :type "HitResult Structure (by ref)"))
  (bind _asbp_paper_zdcharacter (cast `/Game/_Cyberiada/PaperZD/Blueprint/BP_PaperZDCharacter` OtherActor))
  (bind _damage (`/Game/_Cyberiada/PlayerStats/BPC_Stats.getDamage` (`self.BPC_Stats`)))
  (`/Game/_Cyberiada/PlayerStats/BPC_Stats.takeDamage` (`self.GetComponentByClass` _asbp_paper_zdcharacter "/Game/_Cyberiada/PlayerStats/BPC_Stats.BPC_Stats_C") _damage))

(event `self.ReceiveTick`
  (params (DeltaSeconds :type "Float (single-precision)"))
  (bind _returnvalue (`self.K2_GetActorLocation`))
  (bind _returnvalue_2 (`self.K2_GetActorLocation`))
  (bind _returnvalue_3 (`self.K2_GetActorLocation`))
  (`parent.ReceiveTick` DeltaSeconds)
  (if (< (`/Game/_Cyberiada/PlayerStats/BPC_Stats.Hp` (`self.BPC_Stats`)) (* 0.5 (`/Game/_Cyberiada/PlayerStats/BPC_Stats.MaxHp` (`self.BPC_Stats`))))
    (`KismetSystemLibrary.Delay` 3.0)
    (bind _outhit (`KismetSystemLibrary.SphereTraceSingle` _returnvalue _returnvalue 500.0 "TraceTypeQuery1" false (`|MakeArray` self :!type "Actor Object Reference") "ForDuration"))
    (bind _returnvalue_4 (`GameplayStatics.SpawnEmitterAtLocation` "/Game/StarterContent/Particles/P_Sparks.P_Sparks" (`.Location` (`GameplayStatics.BreakHitResult` _outhit)) (struct) (100.0 100.0 100.0)))
    (`KismetSystemLibrary.Delay` 1.0)
    (`ActorComponent.K2_DestroyComponent` _returnvalue_4)
    (elif (< (`/Game/_Cyberiada/PlayerStats/BPC_Stats.Hp` (`self.BPC_Stats`)) (* 0.25 (`/Game/_Cyberiada/PlayerStats/BPC_Stats.MaxHp` (`self.BPC_Stats`))))
      (`KismetSystemLibrary.Delay` 2.0)
      (bind _outhit_2 (`KismetSystemLibrary.SphereTraceSingle` _returnvalue_2 _returnvalue_2 400.0 "TraceTypeQuery1" false (`|MakeArray` self :!type "Actor Object Reference") "ForDuration"))
      (bind _returnvalue_5 (`GameplayStatics.SpawnEmitterAtLocation` "/Game/StarterContent/Particles/P_Fire.P_Fire" (`.Location` (`GameplayStatics.BreakHitResult` _outhit_2)) (struct) (30.0 30.0 30.0)))
      (`KismetSystemLibrary.Delay` 1.0)
      (`ActorComponent.K2_DestroyComponent` _returnvalue_5)
      (else
        (`KismetSystemLibrary.Delay` 3.0)
        (bind _outhit_3 (`KismetSystemLibrary.SphereTraceSingle` _returnvalue_3 _returnvalue_3 300.0 "TraceTypeQuery1" false (`|MakeArray` self :!type "Actor Object Reference") "ForDuration"))
        (bind _returnvalue_6 (`GameplayStatics.SpawnEmitterAtLocation` "/Game/StarterContent/Particles/P_Fire.P_Fire" (`.Location` (`GameplayStatics.BreakHitResult` _outhit_3)) (struct) (30.0 30.0 30.0)))
        (`KismetSystemLibrary.Delay` 1.0)
        (`ActorComponent.K2_DestroyComponent` _returnvalue_6)))))

(fn `UserConstructionScript`
  (`parent.UserConstructionScript`))