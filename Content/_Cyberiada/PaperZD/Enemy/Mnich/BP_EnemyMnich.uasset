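; BP_EnemyMnich is a PaperZD enemy that chases the player, damages characters on hitbox overlap and can heal nearby allies.
; BeginPlay sets its BPC_Stats, starts a looping timer and loops AIMoveTo, destroying itself if dead whenever a move finishes.
; HealAllies sphere-traces around the monk, ignoring the player, and restores HP equal to its Damage stat, with debug drawing on.
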(event `self.ReceiveBeginPlay`
  (bind _bpc_stats (`self.BPC_Stats`))
  (`parent.ReceiveBeginPlay`)
  (bind _returnvalue (`KismetSystemLibrary.K2_SetTimerDelegate` (`|CreateDelegate` :!event `HealAllies`) 3.0 true))
  (set `self.NewVar` _returnvalue)
  (bind _output_get (set `/Game/_Cyberiada/PlayerStats/BPC_Stats.MaxHp` 40 _bpc_stats))
  (set `/Game/_Cyberiada/PlayerStats/BPC_Stats.Hp` _output_get _bpc_stats)
  (set `/Game/_Cyberiada/PlayerStats/BPC_Stats.Damage` 5 _bpc_stats)
  (`|AIMoveTo` self (0.0 0.0 0.0) (`GameplayStatics.GetPlayerCharacter` 0) 100.0 :!label _label
    (:`OnSuccess`
      _)
    (:`OnFail`
      _))
  (bind _isdead (`/Game/_Cyberiada/PlayerStats/BPC_Stats.getIsDead` (`self.BPC_Stats`)))
  (if _isdead
    (`self.K2_DestroyActor`)
    (else
      (goto _label))))

(event `self.HitboxAttak.OnComponentBeginOverlap`
  (params (OverlappedComponent :type "PrimitiveComponent Object Reference") (OtherActor :type "Actor Object Reference") (OtherComp :type "PrimitiveComponent Object Reference") (OtherBodyIndex :type Integer) (bFromSweep :type Boolean) (SweepResult :type "HitResult Structure (by ref)"))
  (bind _asbp_paper_zdcharacter (cast `/Game/_Cyberiada/PaperZD/Blueprint/BP_PaperZDCharacter` OtherActor))
  (bind _damage (`/Game/_Cyberiada/PlayerStats/BPC_Stats.getDamage` (`self.BPC_Stats`)))
  (`/Game/_Cyberiada/PlayerStats/BPC_Stats.takeDamage` (`self.GetComponentByClass` _asbp_paper_zdcharacter "/Game/_Cyberiada/PlayerStats/BPC_Stats.BPC_Stats_C") _damage))

(fn `HealAllies`
  (bind _returnvalue (`self.K2_GetActorLocation`))
  (bind _damage (`/Game/_Cyberiada/PlayerStats/BPC_Stats.getDamage` (`self.BPC_Stats`)))
  (set `self.HealAmount` _damage)
  (bind _outhits (`KismetSystemLibrary.SphereTraceMultiByProfile` _returnvalue _returnvalue 300.0 "BlockAllDynamic" false (`|MakeArray` (`GameplayStatics.GetPlayerCharacter` 0) :!type "Actor Object Reference") "ForDuration" true (struct :`R` 1.0 :`A` 1.0) (struct :`G` 1.0 :`A` 1.0) 0.4))
  (for _array_element _outhits
    (if (`KismetSystemLibrary.IsValid` (`.HitActor` (`GameplayStatics.BreakHitResult` _array_element)))
      (bind _returnvalue_2 (`self.GetComponentByClass` (`.HitActor` (`GameplayStatics.BreakHitResult` _array_element)) "/Game/_Cyberiada/PlayerStats/BPC_Stats.BPC_Stats_C"))
      (if (`KismetSystemLibrary.IsValid` _returnvalue_2)
        (`/Game/_Cyberiada/PlayerStats/BPC_Stats.restoreHp` _returnvalue_2 (`self.HealAmount`))))))

(fn `UserConstructionScript`
  (`parent.UserConstructionScript`))