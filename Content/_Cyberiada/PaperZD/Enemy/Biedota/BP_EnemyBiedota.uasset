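; Biedota enemy Blueprint that chases the player and deals contact damage.
; BeginPlay seeds its stats component, then loops AIMoveTo toward the player, checking for death only when each move succeeds or fails.
; On death it destroys itself, with a small chance to spawn an Apteczka item at its location.
; Its attack hitbox overlap damages any PaperZD character through that character's stats component and calls CheckAlive.
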(event `self.ReceiveBeginPlay`
  (bind _bpc_stats (`self.BPC_Stats`))
  (bind _output_get (set `/Game/_Cyberiada/PlayerStats/BPC_Stats.MaxHp` 65 _bpc_stats))
  (set `/Game/_Cyberiada/PlayerStats/BPC_Stats.Hp` _output_get _bpc_stats)
  (set `/Game/_Cyberiada/PlayerStats/BPC_Stats.Damage` 10 _bpc_stats)
  (`|AIMoveTo` self (0.0 0.0 0.0) (`GameplayStatics.GetPlayerCharacter` 0) 100.0 :!label _label
    (:`OnSuccess`
      _)
    (:`OnFail`
      _))
  (bind _isdead (`/Game/_Cyberiada/PlayerStats/BPC_Stats.getIsDead` (`self.BPC_Stats`)))
  (if _isdead
    (bind _output_get_2 (set `self.Location` (`SceneComponent.K2_GetComponentLocation` (`self.CapsuleComponent`))))
    (`self.K2_DestroyActor`)
    (if (`KismetMathLibrary.RandomBoolWithWeight` 0.1)
      (`|SpawnActorFromClass` "/Game/_Cyberiada/PickableItems/BP_Item_Apteczka.BP_Item_Apteczka_C" (`KismetMathLibrary.Conv_VectorToTransform` _output_get_2) "Undefined" "MultiplyWithRoot" null null))
    (else
      (goto _label))))

(event `self.ReceiveTick`
  (params (DeltaSeconds :type "Float (single-precision)"))
  (`parent.ReceiveTick` DeltaSeconds))

(event `self.HitboxAttak.OnComponentBeginOverlap`
  (params (OverlappedComponent :type "PrimitiveComponent Object Reference") (OtherActor :type "Actor Object Reference") (OtherComp :type "PrimitiveComponent Object Reference") (OtherBodyIndex :type Integer) (bFromSweep :type Boolean) (SweepResult :type "HitResult Structure (by ref)"))
  (bind _asbp_paper_zdcharacter (cast `/Game/_Cyberiada/PaperZD/Blueprint/BP_PaperZDCharacter` OtherActor))
  (bind _damage (`/Game/_Cyberiada/PlayerStats/BPC_Stats.getDamage` (`self.BPC_Stats`)))
  (`/Game/_Cyberiada/PlayerStats/BPC_Stats.takeDamage` (`self.GetComponentByClass` _asbp_paper_zdcharacter "/Game/_Cyberiada/PlayerStats/BPC_Stats.BPC_Stats_C") _damage)
  (`/Game/_Cyberiada/PaperZD/Blueprint/BP_PaperZDCharacter.CheckAlive` _asbp_paper_zdcharacter))

(fn `UserConstructionScript`
  (`parent.UserConstructionScript`))