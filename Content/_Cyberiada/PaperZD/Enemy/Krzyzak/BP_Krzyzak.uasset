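; Krzyzak enemy for the PaperZD game: sets its own health and damage in BPCStats and endlessly chases the player with a re-issued AIMoveTo.
; Its attack hitbox applies the current damage to any overlapping PaperZD character's stats component.
; WasIHurt temporarily boosts damage and lights a PointLight, while Smierc destroys the actor if dead.
; BeginPlay starts two event timers, one looping, and Tick tracks health drops in TempHP.
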(event `Smierc`
  (bind _isdead (`/Game/_Cyberiada/PlayerStats/BPC_Stats.getIsDead` (`self.BPC_Stats`)))
  (if _isdead
    (`self.K2_DestroyActor`)))

(event `self.ReceiveBeginPlay`
  (bind _bpc_stats (`self.BPC_Stats`))
  (`parent.ReceiveBeginPlay`)
  (`KismetSystemLibrary.K2_SetTimerDelegate` (`|CreateDelegate` :!event `WasIHurt`) 0.5)
  (bind _maxhp (`/Game/_Cyberiada/PlayerStats/BPC_Stats.getMaxHp` (`self.BPC_Stats`)))
  (set `self.TempHP` _maxhp)
  (`KismetSystemLibrary.K2_SetTimerDelegate` (`|CreateDelegate` :!event `Smierc`) 0.5 true)
  (bind _output_get (set `/Game/_Cyberiada/PlayerStats/BPC_Stats.MaxHp` 500 _bpc_stats))
  (set `/Game/_Cyberiada/PlayerStats/BPC_Stats.Hp` _output_get _bpc_stats)
  (set `/Game/_Cyberiada/PlayerStats/BPC_Stats.Damage` 35 _bpc_stats)
  (`|AIMoveTo` self (0.0 0.0 0.0) (`GameplayStatics.GetPlayerCharacter` 0) 50.0 :!label _label
    (:`OnSuccess`
      (goto _label))
    (:`OnFail`
      (goto _label))))

(event `self.HitboxAttak.OnComponentBeginOverlap`
  (params (OverlappedComponent :type "PrimitiveComponent Object Reference") (OtherActor :type "Actor Object Reference") (OtherComp :type "PrimitiveComponent Object Reference") (OtherBodyIndex :type Integer) (bFromSweep :type Boolean) (SweepResult :type "HitResult Structure (by ref)"))
  (bind _asbp_paper_zdcharacter (cast `/Game/_Cyberiada/PaperZD/Blueprint/BP_PaperZDCharacter` OtherActor))
  (bind _damage (`/Game/_Cyberiada/PlayerStats/BPC_Stats.getDamage` (`self.BPC_Stats`)))
  (`/Game/_Cyberiada/PlayerStats/BPC_Stats.takeDamage` (`self.GetComponentByClass` _asbp_paper_zdcharacter "/Game/_Cyberiada/PlayerStats/BPC_Stats.BPC_Stats_C") _damage))

(event `WasIHurt`
  (`LightComponent.SetIntensity` (`self.PointLight`) 35000.0)
  (set `/Game/_Cyberiada/PlayerStats/BPC_Stats.Damage` 60 (`self.BPC_Stats`))
  (`KismetSystemLibrary.Delay` 5.0)
  (`LightComponent.SetIntensity` (`self.PointLight`) 0.0)
  (set `/Game/_Cyberiada/PlayerStats/BPC_Stats.Damage` 35 (`self.BPC_Stats`)))

(event `self.ReceiveTick`
  (params (DeltaSeconds :type "Float (single-precision)"))
  (`parent.ReceiveTick` DeltaSeconds)
  (bind _hp (`/Game/_Cyberiada/PlayerStats/BPC_Stats.getHp` (`self.BPC_Stats`)))
  (if (< _hp (`self.TempHP`))
    (set `self.TempHP` (`/Game/_Cyberiada/PlayerStats/BPC_Stats.Hp` (`self.BPC_Stats`)))))

(fn `UserConstructionScript`
  (`parent.UserConstructionScript`))