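; Mafia boss enemy Blueprint in the PaperZD enemy set that periodically summons goons.
; On BeginPlay it runs the parent logic and starts a looping five-second timer, apparently bound to SpawnGoon.
; SpawnGoon picks a random navigable point near the capsule and spawns a BP_EnemyCpun there.
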(event `self.ReceiveBeginPlay`
  (`parent.ReceiveBeginPlay`)
  (`KismetSystemLibrary.K2_SetTimerDelegate` (`|CreateDelegate` :!event `SpawnGoon`) 5.0 true))

(event `SpawnGoon`
  (bind _randomlocation (`NavigationSystemV1.K2_GetRandomLocationInNavigableRadius` (`SceneComponent.K2_GetComponentLocation` (`self.CapsuleComponent`)) 60.0 null null))
  (`|SpawnActorFromClass` "/Game/_Cyberiada/PaperZD/Enemy/Cpun/BP_EnemyCpun.BP_EnemyCpun_C" (`KismetMathLibrary.Conv_VectorToTransform` _randomlocation) "Undefined" "MultiplyWithRoot" null null))

(fn `UserConstructionScript`
  (`parent.UserConstructionScript`))