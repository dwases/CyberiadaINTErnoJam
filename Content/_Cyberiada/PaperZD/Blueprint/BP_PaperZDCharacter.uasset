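; Top-down PaperZD player character with Enhanced Input movement, a melee attack and a toggleable inventory.
; BeginPlay adds the input mapping and seeds BPCStats; movement input also stores Direction.
; Z sphere-traces around the character to damage BPI_Damageable actors, while I creates or removes WBP_Inventory.
; Its health functions use separate CurrHealth/MaxHealth variables rather than BPCStats, and Heal only returns clamped current health, ignoring Amount.
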(event `self.ReceiveTick`
  (params (DeltaSeconds :type "Float (single-precision)")))

(event `self.ReceiveBeginPlay`
  (bind _bpc_stats (`self.BPC_Stats`))
  (bind _asplayer_controller (cast `PlayerController` (`self.GetController`)))
  (bind _returnvalue (pcsubsystem `EnhancedInputLocalPlayerSubsystem` _asplayer_controller))
  (`/Engine/EditorBlueprintResources/StandardMacros.IsValid` _returnvalue
    (:`Is Valid`
      (`EnhancedInputSubsystemInterface.AddMappingContext` _returnvalue "/Game/_Cyberiada/PaperZD/Input/TopDown_IMC.TopDown_IMC" 0 (struct))
      (bind _output_get (set `/Game/_Cyberiada/PlayerStats/BPC_Stats.MaxHp` 100 _bpc_stats))
      (set `/Game/_Cyberiada/PlayerStats/BPC_Stats.Hp` _output_get _bpc_stats)
      (set `/Game/_Cyberiada/PlayerStats/BPC_Stats.Damage` 10 _bpc_stats)
      (set `/Game/_Cyberiada/PlayerStats/BPC_Stats.IsDamagable` true _bpc_stats))))

(event `EnhancedInput|/Game/_Cyberiada/PaperZD/Input/Move_IA`
  (params (ActionValue :type "Vector2D Structure") (ElapsedSeconds :type "Float (double-precision)") (TriggeredSeconds :type "Float (double-precision)") (InputAction :type "InputAction Object Reference" :default "/Game/_Cyberiada/PaperZD/Input/Move_IA.Move_IA"))
  (:`Triggered`
    (`self.AddMovementInput` (1.0 0.0 0.0) ActionValue_X)
    (`self.AddMovementInput` (0.0 1.0 0.0) ActionValue_Y)
    (set `self.Direction` (`KismetMathLibrary.MakeVector2D` ActionValue_X ActionValue_Y))))

(event `Key|Z`
  (params (Key :type "Key Structure"))
  (bind _returnvalue (`self.K2_GetActorLocation`))
  (:`Pressed`
    (bind _outhit (`KismetSystemLibrary.SphereTraceSingle` _returnvalue _returnvalue 90.0 "TraceTypeQuery1" false (`|MakeArray` self :!type "Actor Object Reference") "ForDuration"))
    (bind _asbpi_damageable (cast `/Game/_Cyberiada/DamageSystem/BPI_Damageable` (`.HitActor` (`GameplayStatics.BreakHitResult` _outhit))))
    (`/Game/_Cyberiada/DamageSystem/BPI_Damageable.TakeDamage` _asbpi_damageable (make `/Game/_Cyberiada/DamageSystem/S_DamageInfo` 20.0))))

(event `Key|I`
  (params (Key :type "Key Structure"))
  (:`Pressed`
    (bind _inventorywidget (`self.InventoryWidget`)
      (:`then`
        (`Widget.RemoveFromParent` _inventorywidget)
        (set `self.InventoryWidget` null))
      (:`else`
        (bind _returnvalue (`|CreateWidget` "/Game/_Cyberiada/Widgety/WBP_Inventory.WBP_Inventory_C" null self))
        (`UserWidget.AddToViewport` _returnvalue 0)
        (set `self.InventoryWidget` _returnvalue)))))

(fn `GetCurrentHealth`
  (returns (Health :type "Float (double-precision)"))
  (return (`self.CurrHealth`)))

(fn `GetMaxHealth`
  (returns (MaxHealth :type "Float (double-precision)"))
  (return (`self.MaxHealth`)))

(fn `Heal`
  (params (Amount :type "Float (double-precision)"))
  (returns (NewHealth :type "Float (double-precision)"))
  (return (`KismetMathLibrary.FClamp` (`self.CurrHealth`) 0.0 (`self.MaxHealth`))))

(fn `TakeDamage`
  (params (DamageInfo :type "/Game/_Cyberiada/DamageSystem/S_DamageInfo Structure"))
  (returns (WasDamaged :type Boolean))
  (bind (_amount _shoulddamageinvincible) (break `/Game/_Cyberiada/DamageSystem/S_DamageInfo` DamageInfo))
  (if (not _shoulddamageinvincible)
    (set `self.CurrHealth` (- (`self.CurrHealth`) _amount))
    (return true)
    (else
      (return false))))

(fn `UserConstructionScript`
  (bind _output_get (set `self.MaxHealth` 100.0))
  (set `self.CurrHealth` _output_get))