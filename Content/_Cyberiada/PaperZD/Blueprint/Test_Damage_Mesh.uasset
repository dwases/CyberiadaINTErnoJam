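; Test damage target actor that tracks current and max health through GetCurrentHealth, GetMaxHealth, Heal and TakeDamage functions.
; TakeDamage subtracts the damage amount only when ShouldDamageInvincible is false, printing a Polish debug death message and returning true once health drops below zero.
; Heal only returns current health clamped to the maximum, leaving Amount unapplied and health unchanged.
; Event graph and construction script are empty.
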(fn `GetCurrentHealth`
  (returns (Health :type "Float (double-precision)"))
  (return (`self.CurrHealth`)))

(fn `GetMaxHealth`
  (returns (MaxHealth :type "Float (double-precision)"))
  (return (`self.MaxHealth`)))

(fn `Heal`
  (params (Amount :type "Float (double-precision)"))
  (returns (NewHealth :type "Float (double-precision)"))
  (return (`KismetMathLibrary.FClamp` (`self.CurrHealth`) 0.0 (`self.MaxHealth`))))

(fn `TakeDamage`
  (params (DamageInfo :type "/Game/_Cyberiada/DamageSystem/S_DamageInfo Structure"))
  (returns (WasDamaged :type Boolean))
  (bind (_amount _shoulddamageinvincible) (break `/Game/_Cyberiada/DamageSystem/S_DamageInfo` DamageInfo))
  (if (not _shoulddamageinvincible)
    (set `self.CurrHealth` (- (`self.CurrHealth`) _amount))
    (if (< (`self.CurrHealth`) 0.0)
      (`KismetSystemLibrary.PrintString` "testowy aktor martwy")
      (return true))
    (else
      (return false))))

(fn `UserConstructionScript`)