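; Dungeon boss spawner that starts a timed wave of enemies when the player character enters its trigger box, which then destroys itself.
; A looping timer spawns the configured enemy class at random points around the actor, counting down the remaining total and collecting each enemy's stats component.
; Once the count runs out, a second timer apparently polls those components through OpenDoors, which only clears the timer when none remain valid.
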(event `self.Box.OnComponentBeginOverlap`
  (params (OverlappedComponent :type "PrimitiveComponent Object Reference") (OtherActor :type "Actor Object Reference") (OtherComp :type "PrimitiveComponent Object Reference") (OtherBodyIndex :type Integer) (bFromSweep :type Boolean) (SweepResult :type "HitResult Structure (by ref)"))
  (cast `/Game/_Cyberiada/PaperZD/Blueprint/BP_PaperZDCharacter` OtherActor)
  (`KismetSystemLibrary.PrintString` (`KismetSystemLibrary.GetDisplayName` OtherComp))
  (`ActorComponent.K2_DestroyComponent` (`self.Box`))
  (bind _returnvalue (`KismetSystemLibrary.K2_SetTimerDelegate` (`|CreateDelegate` :!event `Spawn`) 2.0 true))
  (set `self.Timer` _returnvalue))

(event `Spawn`
  (bind _iloscwrogow (`self.IloscWrogow`))
  (bind (_returnvalue_x _returnvalue_y) (`KismetMathLibrary.BreakVector` (`KismetMathLibrary.RandomPointInBoundingBox` (`self.K2_GetActorLocation`) (650.0 650.0 0.0))))
  (bind _returnvalue (`|SpawnActorFromClass` (`self.EnemyClass`) (`KismetMathLibrary.MakeTransform` (`KismetMathLibrary.MakeVector` _returnvalue_x _returnvalue_y 20.0)) "AlwaysSpawn" "MultiplyWithRoot" null null))
  (`|ExecutionSequence`
    (:`then_0`
      (`/Engine/EditorBlueprintResources/StandardMacros.DecrementInt` _iloscwrogow
        (:`  `
          (if (<= _iloscwrogow 0)
            (`KismetSystemLibrary.K2_ClearAndInvalidateTimerHandle` (`self.Timer`))
            (bind _returnvalue_2 (`KismetSystemLibrary.K2_SetTimerDelegate` (`|CreateDelegate` :!event `OpenDoors`) 1.0 true))
            (set `self.Timer` _returnvalue_2)))))
    (:`then_1`
      (`KismetArrayLibrary.Array_Add` (`self.Wrogowie`) (`self.GetComponentByClass` _returnvalue "/Game/_Cyberiada/PlayerStats/BPC_Stats.BPC_Stats_C")))))

(event `OpenDoors`
  (set `self.IsAlive` false)
  (for _array_element (`self.Wrogowie`)
    (set `self.IsAlive` (or (`KismetSystemLibrary.IsValid` _array_element) (`self.IsAlive`))))
  (if (not (`self.IsAlive`))
    (`KismetSystemLibrary.K2_ClearAndInvalidateTimerHandle` (`self.Timer`))))

(fn `UserConstructionScript`)