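; Pickable first-aid kit item that restores a fixed amount of HP to the player.
; On any actor overlap it casts the player pawn, not the overlapping actor, to BP_PaperZDCharacter and calls RestoreHp on its BPCStats component.
; It prints the HP read before healing, then calls the parent overlap handler; if the cast fails, neither healing nor the parent call runs.
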(event `self.ReceiveActorBeginOverlap`
  (params (OtherActor :type "Actor Object Reference"))
  (bind _asbp_paper_zdcharacter (cast `/Game/_Cyberiada/PaperZD/Blueprint/BP_PaperZDCharacter` (`GameplayStatics.GetPlayerPawn` 0)))
  (bind _bpc_stats (`/Game/_Cyberiada/PaperZD/Blueprint/BP_PaperZDCharacter.BPC_Stats` _asbp_paper_zdcharacter))
  (bind _hp (`/Game/_Cyberiada/PlayerStats/BPC_Stats.getHp` _bpc_stats))
  (`KismetSystemLibrary.PrintString` (`KismetStringLibrary.Conv_IntToString` _hp))
  (`/Game/_Cyberiada/PlayerStats/BPC_Stats.restoreHp` _bpc_stats 10)
  (`/Game/_Cyberiada/PlayerStats/BPC_Stats.getHp` _bpc_stats)
  (`parent.ReceiveActorBeginOverlap` OtherActor))

(fn `UserConstructionScript`
  (`parent.UserConstructionScript`))