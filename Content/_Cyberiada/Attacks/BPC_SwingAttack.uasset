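; BPC_SwingAttack is an unfinished component for a swing attack fanned out in front of its owner.
; Left mouse press runs a loop from one to SwingDensity, but the loop body is empty.
; A disconnected visibility line trace starts at the owner's location.
; Unused math spreads points at SwingRange across SwingAngle, centred on the owner's facing, apparently intended as trace end points.
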(event `Key|LeftMouseButton`
  (params (Key :type "Key Structure"))
  (:`Pressed`
    (for _index (range 1 (+ (`self.SwingDensity`) 1))
      _)))