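; BP_ArrowProjectile is an arrow projectile that destroys any Pawn it hits.
; It moves through a ProjectileMovement component, and its StaticMesh hit event sets InitialSpeed to zero, leaving current velocity untouched.
; A Pawn hit destroys both the Pawn and the arrow immediately, with no damage call.
; Any other hit destroys the arrow after a short delay.
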(event `self.ReceiveBeginPlay`
  (`parent.ReceiveBeginPlay`))

(event `self.StaticMesh.OnComponentHit`
  (params (HitComponent :type "PrimitiveComponent Object Reference") (OtherActor :type "Actor Object Reference") (OtherComp :type "PrimitiveComponent Object Reference") (NormalImpulse :type "Vector Structure") (Hit :type "HitResult Structure (by ref)"))
  (set `ProjectileMovementComponent.InitialSpeed` 0.0 (`self.ProjectileMovement`))
  (bind _aspawn (cast `Pawn` OtherActor)
    (:`then`
      (`self.K2_DestroyActor` _aspawn))
    (:`CastFailed`
      (`KismetSystemLibrary.Delay` 2.0)))
  (`self.K2_DestroyActor`))

(fn `UserConstructionScript`
  (`parent.UserConstructionScript`))