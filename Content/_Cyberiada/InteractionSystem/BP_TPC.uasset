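; Player pawn Blueprint, likely a third-person character, that toggles a dialog box when E is pressed near an interactable.
; E removes any open dialog; otherwise it runs a debug-drawn sphere trace forward from the actor over InteractRange.
; A hit actor implementing BPI_Interactable opens WBP_Dialog with hard-coded placeholder text, stored in WidgetRef for closing.
; The interface serves only as a filter, with none of its functions called.
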(event `Key|E`
  (params (Key :type "Key Structure"))
  (bind _returnvalue (`self.K2_GetActorLocation`))
  (bind _widgetref (`self.WidgetRef`))
  (:`Pressed`
    (if (`KismetSystemLibrary.IsValid` _widgetref)
      (`Widget.RemoveFromParent` _widgetref)
      (set `self.WidgetRef` null)
      (else
        (bind _outhit (`KismetSystemLibrary.SphereTraceSingle` _returnvalue (+ (* (`KismetMathLibrary.GreaterGreater_VectorRotator` (1.0 0.0 0.0) (`self.K2_GetActorRotation`)) (`self.InteractRange`)) _returnvalue) 60.0 "TraceTypeQuery1" false (`|MakeArray` self :!type "Actor Object Reference") "ForDuration" true (struct :`R` 1.0 :`A` 1.0) (struct :`G` 1.0 :`A` 1.0) 2.0))
        (cast `/Game/_Cyberiada/InteractionSystem/BPI_Interactable` (`.HitActor` (`GameplayStatics.BreakHitResult` _outhit)))
        (bind _returnvalue_2 (`|CreateWidget` "/Game/_Cyberiada/Widgety/WBP_Dialog.WBP_Dialog_C" (`GameplayStatics.GetPlayerController` 0) " \n \nLorem ipsum dolor sit amet, consectetur adipiscing elit. Etiam est arcu, convallis sit amet quam nec, suscipit dignissim felis. Vestibulum laoreet hendrerit ex sit amet finibus. In cursus risus eget nunc volutpat, eget laoreet tortor auctor. Cras mi sem, tempus sit amet suscipit ut, euismod nec nulla. Sed sed tortor dignissim, congue risus eget, ultrices quam. Nulla tempus nulla vitae varius dictum. Nunc condimentum molestie eros, nec venenatis lectus rutrum sit amet. Pellentesque id dictum enim. Morbi maximus nisl purus, non bibendum felis euismod quis. Ut non eleifend nisi. Maecenas bibendum, diam a malesuada porttitor, felis lectus viverra neque, sed pulvinar felis augue iaculis diam. Sed ullamcorper nisl ut nunc vulputate dictum. Proin vehicula enim elit. Nam non libero mollis, eleifend arcu vitae, sagittis nisl. Integer eleifend elit eget nisi dignissim, quis egestas ante rutrum. \n \nSed mattis lorem libero, in vehicula elit ullamcorper et. Donec sollicitudin, massa in ultricies blandit, metus ante venenatis tortor, eget molestie dolor nisl ut mi. Nullam vitae eros quis turpis pulvinar lacinia. Duis aliquet laoreet sapien ut euismod. Vivamus bibendum mauris at feugiat tincidunt. In et magna metus. Morbi ac magna neque. Praesent pulvinar nisl a aliquam malesuada. Interdum et malesuada fames ac ante ipsum. "))
        (`UserWidget.AddToViewport` _returnvalue_2 0)
        (set `self.WidgetRef` _returnvalue_2)))))

(fn `UserConstructionScript`
  (`parent.UserConstructionScript`))