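; Dialog trigger that plays the Polish-language mission briefing in which the King and Trurl send the knight through a portal to eliminate targets in the past.
; BeginPlay writes the hardcoded lines, including a {name} placeholder, into BPCInteractable's Message.
; When BP_PaperZDCharacter overlaps it, the trigger removes any existing widget and passes Message to the character's CreateDialog.
; Nothing disables the trigger, so each new overlap restarts the dialog.
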(event `self.ReceiveBeginPlay`
  (set `/Game/_Cyberiada/InteractionSystem/BPC_Interactable.Message` (`|MakeArray` "KRÓL  \n*zza drzwi * \nJuż posłałem po naszego największego wojownika, na pewno sobie poradzi, w końcu nie raz dowiódł swej wartości. A skoro poradził sobie teraz, to z pewnością poradzi sobie przed naszymi czasami." "KRÓL  \nO wilku mowa! Oczekiwaliśmy Cię... {name}. Trurl wprowadzi Cię w zadanie. " "TRURL  \nW wyniku badań naszego działu analizy przeszłości wytypowaliśmy trzy osoby mające największy wpływ na ograniczenia rozwojowe naszego państwa. Chcemy Cię wysłać w przeszłość w celu wyeliminowania tych ograniczeń." "RYCERZ  \nW sensie... mam ich zabić?" "TRULR  \nNie traktuj ich jak ludzi, są siłą żywą przeciwnika, są jak paproch, rzecz. Stali się nimi kiedy zdecydowaliśmy, że są naszym celem. Patrz tam. " "TRULR  \nTo świecące to portal prowadzący do pierwszej lokacji. Rozpoznasz cel po tym, że będzie się wyjątkowo różnił od innych i będzie głęboko schowany. Przez portal przejść może jedynie tkanka żywa, oparta na atomach biogennych i kilku innych kluczowych dla oddychania. Dlatego kazaliśmy Ci założyć ów skórę pochodzenia zwierzęcego. Niestety, oznacza to, że idziesz tam nie tylko bez zbroi, ale i bez broni. Powodzenia, wojowniku.") (`self.BPC_Interactable`)))

(event `self.ReceiveActorBeginOverlap`
  (params (OtherActor :type "Actor Object Reference"))
  (if true
    (bind _asbp_paper_zdcharacter (cast `/Game/_Cyberiada/PaperZD/Blueprint/BP_PaperZDCharacter` OtherActor))
    (bind _widgetref (`/Game/_Cyberiada/PaperZD/Blueprint/BP_PaperZDCharacter.WidgetRef` _asbp_paper_zdcharacter))
    (if (`KismetSystemLibrary.IsValid` _widgetref)
      (`Widget.RemoveFromParent` _widgetref)
      (set `/Game/_Cyberiada/PaperZD/Blueprint/BP_PaperZDCharacter.WidgetRef` null _asbp_paper_zdcharacter))
    (`/Game/_Cyberiada/PaperZD/Blueprint/BP_PaperZDCharacter.CreateDialog` _asbp_paper_zdcharacter (`/Game/_Cyberiada/InteractionSystem/BPC_Interactable.Message` (`self.BPC_Interactable`)))))

(fn `UserConstructionScript`)